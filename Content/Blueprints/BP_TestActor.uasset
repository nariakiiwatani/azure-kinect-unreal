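; Test actor that visualizes Azure Kinect body tracking as 26 joint components.
; BeginPlay opens the live device or loads a playback file, and EndPlay shuts the device down.
; Tick takes the first tracked body, set to mirrored, retrying until one exists, and copies each joint's position and orientation onto the matching component.
; The construction script fills the component array in joint-index order, so array index maps directly to Kinect joint.
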(event EventBeginPlay
  (if (Variables|Default|GetPlaybackMode)
    (bind _deviceid (Class|AzureKinectManager|LoadfromFile (Utilities|Struct|BreakFilePath (Variables|Default|GetPlaybackFile))))
    (Variables|Default|SetDeviceID _deviceid)
    (else
      (Class|AzureKinectManager|InitDevice (Variables|Default|GetDeviceID) "NFOV_UNBINNED" 33)))
  (Development|PrintString "Initializing Azure Kinect" true true "(R=0.000000,G=0.660000,B=1.000000,A=1.000000)" 1e+01)
  (Class|AzureKinectManager|ToggleDeviceLogging (Variables|Default|GetDeviceID) false true)
  (if (> (Utilities|Array|Length (Class|AzureKinectManager|GetBodies (Variables|Default|GetDeviceID))) 0)
    (bind _output_get (Variables|Default|SetKinectBody (Utilities|Array|Get(acopy) (Class|AzureKinectManager|GetBodies (Variables|Default|GetDeviceID)))))
    (Variables|/Script/AzureKinectUnreal.AzureKinectBody|SetbIsMirrored _output_get true)))

(event Collision|EventActorBeginOverlap
  (params (OtherActor :type Actor%20Object%20Reference)))

(event EventTick
  (params (DeltaSeconds :type Float%20%28single-precision%29))
  (bind _deviceid (Variables|Default|GetDeviceID))
  (bind _returnvalue (Class|AzureKinectManager|GetBodies _deviceid))
  (Variables|Default|GetKinectBody
    (:then
      (Variables|Default|SetKinectJoints (Class|AzureKinectBody|GetJoints (Variables|Default|GetKinectBody)) :!label _label)
      (for (_array_element _array_index) (Variables|Default|GetVisualJoints)
        (Transformation|SetRelativeLocationAndRotation _array_element (.Position (Utilities|Struct|BreakAzureKinectJoint (Utilities|Array|Get(acopy) (Variables|Default|GetKinectJoints) _array_index))) (.Orientation (Utilities|Struct|BreakAzureKinectJoint (Utilities|Array|Get(acopy) (Variables|Default|GetKinectJoints) _array_index))) false false)))
    (:else
      (if (> (Utilities|Array|Length _returnvalue) 0)
        (bind _output_get (Variables|Default|SetKinectBody (Utilities|Array|Get(acopy) _returnvalue)))
        (Utilities|IsValid _output_get
          (:Is%20Valid
            (Variables|/Script/AzureKinectUnreal.AzureKinectBody|SetbIsMirrored _output_get true)
            (goto _label)))))))

(event EventEndPlay
  (params (EndPlayReason :type EEndPlayReason%20Enum :default "Destroyed"))
  (Class|AzureKinectManager|ShutdownDevice (Variables|Default|GetDeviceID)))

(fn ConstructionScript
  (Variables|Default|SetVisualJoints (Utilities|Array|MakeArray (Variables|Default|Get0_Pelvis) (Variables|Default|Get1_SpineNaval) (Variables|Default|Get2_SpineChest) (Variables|Default|Get3_Neck) (Variables|Default|Get4_ClavicleLeft) (Variables|Default|Get5_ShoulderLeft) (Variables|Default|Get6_ElbowLeft) (Variables|Default|Get7_WristLeft) (Variables|Default|Get8_ClavicleRight) (Variables|Default|Get9_ShoulderRight) (Variables|Default|Get10_ElbowRight) (Variables|Default|Get11_WristRight) (Variables|Default|Get12_HipLeft) (Variables|Default|Get13_KneeLeft) (Variables|Default|Get14_AnkleLeft) (Variables|Default|Get15_FootLeft) (Variables|Default|Get16_HipRight) (Variables|Default|Get17_KneeRight) (Variables|Default|Get18_AnkleRight) (Variables|Default|Get19_FootRight) (Variables|Default|Get20_Head) (Variables|Default|Get21_Nose) (Variables|Default|Get22_EyeLeft) (Variables|Default|Get23_EarLeft) (Variables|Default|Get24_EyeRight) (Variables|Default|Get25_EarRight))))